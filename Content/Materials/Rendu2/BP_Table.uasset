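; BP_Table is a table actor whose mesh material animates a dissolve effect when a Pawn overlaps its Box trigger.
; On BeginPlay it creates a dynamic material instance from the StaticMesh's first material and assigns it back to that slot.
; The overlap plays DissolvreTimeline, whose Dissolve track drives the material's Progress scalar parameter while printing the value for debugging.
; The timeline only plays forward, with no handling for the end of the overlap.
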(event OnComponentBeginOverlap(Box)
  (params (OverlappedComponent :type Primitive%20Component%20Object%20Reference) (OtherActor :type Actor%20Object%20Reference) (OtherComp :type Primitive%20Component%20Object%20Reference) (OtherBodyIndex :type Integer) (bFromSweep :type Boolean) (SweepResult :type Hit%20Result%20Structure%20%28by%20ref%29))
  (Utilities|Casting|CastToPawn OtherActor)
  (bind _dissolve (Timeline|DissolvreTimeline Play)
    (:Update
      (Development|PrintString (Utilities|String|ToString(Float) (Math|Float|Lerp 0.0 1.0 _dissolve)))
      (Rendering|Material|SetScalarParameterValue (Variables|Default|GetDynamicMaterialRef) "Progress" (Math|Float|Lerp 0.0 1.0 _dissolve) :!class /Script/Engine.MaterialInstanceDynamic))))

(event EventBeginPlay
  (bind _returnvalue (Rendering|Material|CreateDynamicMaterialInstance (Rendering|Material|GetMaterial (Variables|Default|GetStaticMesh) 0) "None" "None" :!class /Script/Engine.KismetMaterialLibrary))
  (bind _output_get (Variables|Default|SetDynamicMaterialRef _returnvalue))
  (Rendering|Material|SetMaterial (Variables|Default|GetStaticMesh) 0 _output_get))

(fn ConstructionScript)